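; BP_trashMob is a basic enemy with a floating health widget that shows while the player overlaps its SeeHealth volume.
; BeginPlay caches the player and widget references.
; Taking damage spawns a BP_DmgAmount actor and refreshes the widget from MobHealth, which this graph never changes.
; Melee applies random ranged damage directly to the cached player and calls its HUD update with zero values; the loot drop on destruction is an empty stub.
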(event OnComponentEndOverlap(SeeHealth)
  (params (OverlappedComponent :type Primitive%20Component%20Object%20Reference) (OtherActor :type Actor%20Object%20Reference) (OtherComp :type Primitive%20Component%20Object%20Reference) (OtherBodyIndex :type Integer))
  ;[1 1 1] Visibility - Elliot
  (Utilities|Casting|CastToPlayerCharacterBP OtherActor)
  (Rendering|SetVisibility (Variables|Default|GetHealth%20Widget) false false))

(event OnComponentBeginOverlap(SeeHealth)
  (params (OverlappedComponent :type Primitive%20Component%20Object%20Reference) (OtherActor :type Actor%20Object%20Reference) (OtherComp :type Primitive%20Component%20Object%20Reference) (OtherBodyIndex :type Integer) (bFromSweep :type Boolean) (SweepResult :type Hit%20Result%20Structure%20%28by%20ref%29))
  ;[1 1 1] Visibility - Elliot
  (Utilities|Casting|CastToPlayerCharacterBP OtherActor)
  (Rendering|SetVisibility (Variables|Default|GetHealth%20Widget) true false))

(event EventBeginPlay
  ;[1 1 1] Casting so the player can see the ai health widget - Elliot
  (bind _asplayer_character_bp (Utilities|Casting|CastToPlayerCharacterBP (Game|GetPlayerCharacter 0)))
  (Variables|Default|SetPlayerRef _asplayer_character_bp)
  (bind _asw_trash_mob_floating_health (Utilities|Casting|CastToW_TrashMobFloatingHealth (UserInterface|GetUserWidgetObject (Variables|Default|GetHealth%20Widget))))
  (Variables|Default|SetHealth%20Widget%20Ref _asw_trash_mob_floating_health))

(event Collision|EventActorBeginOverlap
  (params (OtherActor :type Actor%20Object%20Reference)))

(event EventMelee
  (bind _returnvalue (Game|Damage|ApplyDamage (Variables|Default|GetPlayerRef) (Math|Random|RandomFloatinRange (Variables|Default|GetMinDamage) (Variables|Default|GetMaxDamage)) 0 self))
  (Default|UpdateHealth (Variables|/Game/Blueprints/Player/PlayerCharacterBP.PlayerCharacterBP_C|GetHealthHudRef (Variables|Default|GetPlayerRef)) 0.0 0.0))

(event EventTick
  (params (DeltaSeconds :type Float%20%28single-precision%29)))

(event Game|Damage|EventAnyDamage
  (params (Damage :type Float%20%28single-precision%29) (DamageType :type Damage%20Type%20Object%20Reference) (InstigatedBy :type Controller%20Object%20Reference) (DamageCauser :type Actor%20Object%20Reference))
  ;[1 1 1] Update Ai Health - Elliot
  (Game|SpawnActorfromClass "/Game/Blueprints/Enemies/Enemy_FloatingHealthWidget/BP_DmgAmount.BP_DmgAmount_C" (Transformation|GetActorTransform) "Undefined" 0 Damage 0)
  (Default|UpdateMobHealth (Variables|Default|GetHealth%20Widget%20Ref) (Variables|Default|GetMobHealth) (Variables|Default|GetMobDefaultHealth)))

(event EventDestroyed
  ;[1 1 1] Drop loot _Elliot
  (if (Variables|Default|GetbIsDead)
    _))

(fn ConstructionScript)