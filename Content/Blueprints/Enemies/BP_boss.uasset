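; Boss enemy character with two attacks, an airstrike barrage and a jump slam, exposed as custom events.
; Ranged uses a delayed loop to spawn BP_airstrike at the player's current X/Y until Count runs out, then resets Count.
; JumpAttack triggers a short jump.
; Any landing fires a heavy camera shake and a tinted ripple widget that a timeline scales before resetting its size.
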(event EventRanged
  (bind _returnvalue (Game|GetPlayerCharacter 0))
  (bind _returnvalue_2 (Transformation|GetActorLocation _returnvalue))
  ;[1 1 1] Airstrike Attack
  (if (> (Variables|Default|GetCount) 0) :!label _label
    (Game|SpawnActorfromClass "/Game/Blueprints/Enemies/BP_airstrike.BP_airstrike_C" (Math|Transform|MakeTransform (Math|Vector|MakeVector (.x _returnvalue_2) (.y _returnvalue_2) 0.0) "0, 0, 0" "1.000000,1.000000,1.000000") "Undefined" 0 0)
    (Variables|Default|SetCount (- (Variables|Default|GetCount) 1))
    (Utilities|FlowControl|Delay 0.5)
    (goto _label)
    (else
      (Variables|Default|SetCount 10))))

(event EventJumpAttack
  ;[1 1 1] Jump Attack
  (Character|Jump)
  (Utilities|FlowControl|Delay 0.1)
  (Character|StopJumping))

(event EventOnLanded
  (params (Hit :type Hit%20Result%20Structure%20%28by%20ref%29))
  ;[1 1 1] Jump Attack
  (Class|MatineeCameraShake|StartMatineeCameraShake (Game|GetPlayerCameraManager 0) "/Game/Blueprints/Enemies/BP_cameraShake.BP_cameraShake_C" 2e+01 "World" "0, 0, 0")
  (Class|WidgetComponent|SetTintColorandOpacity (Variables|Default|GetWidget) (Utilities|Struct|MakeLinearColor 0.0 0.0 1.0 1.0))
  (bind _scale (Timeline|Ripple%20Scale PlayFromStart)
    (:Update
      (Transformation|SetRelativeScale3D (Variables|Default|GetWidget) (Math|Vector|MakeVector _scale _scale _scale)))
    (:Finished
      (Transformation|SetRelativeScale3D (Variables|Default|GetWidget) (Math|Vector|MakeVector 0.2 0.2 0.2)))))

(fn ConstructionScript)