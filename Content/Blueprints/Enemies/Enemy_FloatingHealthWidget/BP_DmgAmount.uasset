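; BP_DmgAmount is a floating damage-number actor, filed with the enemy floating health widget assets.
; On BeginPlay it passes its DmgAmount to the W_DmgAmt widget in its Widget component, stopping if that cast fails.
; The MoveT timeline then lerps the actor from its start location to a fixed raised, sideways world-space offset, and destroys it when finished.
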(event EventBeginPlay
  (bind _asw_dmg_amt (Utilities|Casting|CastToW_DmgAmt (UserInterface|GetWidget (Variables|Default|GetWidget))))
  (Variables|/Game/Blueprints/Enemies/Enemy_FloatingHealthWidget/W_DmgAmt.W_DmgAmt_C|SetDmgAmount _asw_dmg_amt (Variables|Default|GetDmg%20Amount))
  (bind _output_get (Variables|Default|SetStartLocation (Transformation|GetActorLocation)))
  (Variables|Default|SetEnd%20Loc (+ _output_get "-25.000000,-25.000000,75.000000"))
  (bind _move_track (Timeline|Move%20T Play)
    (:Update
      (Transformation|SetActorLocation (Math|Vector|Lerp(Vector) (Variables|Default|GetStartLocation) (Variables|Default|GetEnd%20Loc) _move_track) false false))
    (:Finished
      (Actor|DestroyActor))))

(fn ConstructionScript)