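; Player character Blueprint that creates the ammo, hit box, health and stamina HUD widgets at BeginPlay.
; HealthComp values feed the health HUD on damage, on health increase and twice every Tick without validity checks.
; The damage and health-increase events add a HealthComponent if the reference is invalid.
; Stamina is unfinished: its event sends zeros, StaminaComp is unused, and shotgun ammo HUD creation is disconnected.
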(event EventBeginPlay
  (Utilities|FlowControl|Sequence
    (:then_1
      (bind _returnvalue (UserInterface|CreateWidget "/Game/Widgets/AmmoHud.AmmoHud_C"))
      (UserInterface|Viewport|AddtoViewport _returnvalue 0)
      ;[1 1 1] HitBox
      (bind _returnvalue_2 (UserInterface|CreateWidget "/Game/Widgets/HitBox.HitBox_C"))
      (UserInterface|Viewport|AddtoViewport _returnvalue_2 0)
      ;[1 1 1] HealthHud
      (bind _returnvalue_3 (UserInterface|CreateWidget "/Game/Widgets/HealthHud.HealthHud_C"))
      (bind _output_get (Variables|Default|SetHealthHudRef _returnvalue_3))
      (UserInterface|Viewport|AddtoViewport _output_get 0)
      ;[1 1 1] Stamina Hud
      (bind _returnvalue_4 (UserInterface|CreateWidget "/Game/Widgets/StaminaHud.StaminaHud_C"))
      (bind _output_get_2 (Variables|Default|SetStaminaHudRef _returnvalue_4))
      (UserInterface|Viewport|AddtoViewport _output_get_2 0))))

(event EventIncreaseHealth
  (params (OtherActor :type Health%20Component%20Object%20Reference))
  ;[1 1 1] On pickup increase health
  (Utilities|IsValid (Variables|Default|GetHealthHudRef)
    (:Is%20Valid
      (Utilities|IsValid (Variables|Default|GetHealthComp)
        (:Is%20Valid
          _)
        (:Is%20Not%20Valid
          (bind _returnvalue (Game|AddComponentbyClass "/Script/BSca_Y2T2J.HealthComponent"))
          (Variables|Default|SetHealthComp _returnvalue)))
      (Default|UpdateHealth (Variables|Default|GetHealthHudRef) (Variables|/Script/BSca_Y2T2J.HealthComponent|GetHealth (Variables|Default|GetHealthComp)) (Variables|/Script/BSca_Y2T2J.HealthComponent|GetDefaultHealth (Variables|Default|GetHealthComp))))))

(event Game|Damage|EventAnyDamage
  (params (Damage :type Float%20%28single-precision%29) (DamageType :type Damage%20Type%20Object%20Reference) (InstigatedBy :type Controller%20Object%20Reference) (DamageCauser :type Actor%20Object%20Reference))
  ;[1 1 1] Checks On damage if valid
  (Utilities|IsValid (Variables|Default|GetHealthHudRef)
    (:Is%20Valid
      (Utilities|IsValid (Variables|Default|GetHealthComp)
        (:Is%20Valid
          _)
        (:Is%20Not%20Valid
          (bind _returnvalue (Game|AddComponentbyClass "/Script/BSca_Y2T2J.HealthComponent"))
          (Variables|Default|SetHealthComp _returnvalue)))
      (Default|UpdateHealth (Variables|Default|GetHealthHudRef) (Variables|/Script/BSca_Y2T2J.HealthComponent|GetHealth (Variables|Default|GetHealthComp)) (Variables|/Script/BSca_Y2T2J.HealthComponent|GetDefaultHealth (Variables|Default|GetHealthComp))))))

(event EventOnStaminaUse
  ;[1 1 1] On Run
  (Utilities|IsValid (Variables|Default|GetStaminaHudRef)
    (:Is%20Valid
      (Default|UpdateStamina (Variables|Default|GetStaminaHudRef) 0.0 0.0))))

(event EventTick
  (params (DeltaSeconds :type Float%20%28single-precision%29))
  (bind _healthcomp (Variables|Default|GetHealthComp))
  (bind _healthcomp_2 (Variables|Default|GetHealthComp))
  (Utilities|FlowControl|Sequence
    (:then_0
      ;[1 1 1] Checks On damage if valid
      (Default|UpdateHealth (Variables|Default|GetHealthHudRef) (Variables|/Script/BSca_Y2T2J.HealthComponent|GetHealth _healthcomp) (Variables|/Script/BSca_Y2T2J.HealthComponent|GetDefaultHealth _healthcomp)))
    (:then_1
      ;[1 1 1] On pickup increase health
      (Default|UpdateHealth (Variables|Default|GetHealthHudRef) (Variables|/Script/BSca_Y2T2J.HealthComponent|GetHealth _healthcomp_2) (Variables|/Script/BSca_Y2T2J.HealthComponent|GetDefaultHealth _healthcomp_2)))))

(fn ConstructionScript)